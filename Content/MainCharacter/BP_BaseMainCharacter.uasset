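; BP_BaseMainCharacter is the base Blueprint for the main character, adding camera shake that matches its movement state.
; Every tick it chooses an idle, walk or sprint shake from its velocity and the sprint state reported by PlayerMovementComponent.
; SetCameraShake starts that shake on the controlling PlayerController's camera manager, issuing a new start call each frame.
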(event Custom|ChangeCameraShake
  (if (not (Math|Vector|VectorIsZero (Transformation|GetVelocity)))
    (if (not (Class|PlayerMovementComponent|IsPlayerSprinting (Variables|Default|GetPlayerMovementComponent)))
      (CallFunction|SetCameraShake (Variables|Default|GetWalkCameraShake))
      (else
        (CallFunction|SetCameraShake (Variables|Default|GetSprintCameraShake))))
    (else
      (CallFunction|SetCameraShake (Variables|Default|GetCameraShakeIdle)))))

(event EventTick
  (params (DeltaSeconds :type Float%20%28single-precision%29))
  (CallFunction|ChangeCameraShake))

(fn ConstructionScript)

(fn SetCameraShake
  (params (ShakeClass :type Camera%20Shake%20Base%20Class%20Reference))
  (bind _asplayer_controller (Utilities|Casting|CastToPlayerController (Pawn|GetController)))
  (CameraShakes|StartCameraShake (Variables|/Script/Engine.PlayerController|GetPlayerCameraManager _asplayer_controller) ShakeClass 1.0 "CameraLocal" "0, 0, 0"))